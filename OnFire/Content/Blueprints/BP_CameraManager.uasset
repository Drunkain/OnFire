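; Camera manager actor that serves as the player's view and moves between preset camera positions as the fire's strength changes.
; On BeginPlay it finds the BP_CameraPositionsHandler, becomes the view target and snaps into place.
; Every tick it reads FireStrength from BP_FeuerGM's fire and finds the two cameras bracketing it, treating array order as evenly spaced thresholds.
; It lerps between their transforms and eases toward the result with TInterpTo.
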(event `self.ReceiveBeginPlay`
  (bind _outactors (`GameplayStatics.GetAllActorsOfClass` "/Game/Blueprints/BP_CameraPositionsHandler.BP_CameraPositionsHandler_C"))
  (set `self.CamPosHandler` (`|GetArrayItem` _outactors))
  (`PlayerController.SetViewTargetWithBlend` (`GameplayStatics.GetPlayerController` 0) self 0.0 "VTBlend_Linear" 0.0 false)
  (`self.UpdateCameraTransform` (`GameplayStatics.GetWorldDeltaSeconds`) true))

(event `self.ReceiveTick`
  (params (DeltaSeconds :type "Float (single-precision)"))
  (`self.UpdateCameraTransform` DeltaSeconds))

(fn `UpdateCameraTransform`
  (params (Delta :type "Float (double-precision)") (NoInterp :type Boolean))
  (locals (CamRatio :type "Float (double-precision)") (CurrentFireStrength :type "Float (double-precision)") (LowIndex :type Integer) (HighIndex :type Integer) (HighTransform :type "Transform Structure") (LowTransform :type "Transform Structure"))
  (bind _returnvalue (`self.GetTransform`))
  (bind _returnvalue_2 (`KismetMathLibrary.Conv_IntToDouble` (`KismetArrayLibrary.Array_Length` (`/Game/Blueprints/BP_CameraPositionsHandler.Cameras` (`self.CamPosHandler`)))))
  (bind _returnvalue_3 (`KismetMathLibrary.TLerp` (`local.LowTransform`) (`local.HighTransform`) (`KismetMathLibrary.MapRangeClamped` (`local.CurrentFireStrength`) (/ (`KismetMathLibrary.Conv_IntToDouble` (`local.LowIndex`)) _returnvalue_2) (/ (`KismetMathLibrary.Conv_IntToDouble` (`local.HighIndex`)) _returnvalue_2) 0.0 1.0)))
  (set `local.HighTransform` _returnvalue)
  (set `local.LowTransform` _returnvalue)
  (bind _asbp_feuer_gm (cast `/Game/Blueprints/BP_FeuerGM` (`GameplayStatics.GetGameMode`)))
  (set `local.CurrentFireStrength` (`/Game/Blueprints/BP_Fire.FireStrength` (`/Game/Blueprints/BP_FeuerGM.FireRef` _asbp_feuer_gm)))
  (for (_array_element _array_index) (`/Game/Blueprints/BP_CameraPositionsHandler.Cameras` (`self.CamPosHandler`))
    (if (<= (`local.CurrentFireStrength`) (/ (`KismetMathLibrary.Conv_IntToDouble` _array_index) (`KismetMathLibrary.Conv_IntToDouble` (`KismetArrayLibrary.Array_Length` (`/Game/Blueprints/BP_CameraPositionsHandler.Cameras` (`self.CamPosHandler`))))))
      (set `local.HighIndex` _array_index)
      (bind _returnvalue_4 (`self.GetTransform` _array_element))
      (set `local.HighTransform` _returnvalue_4)
      (break)
      (else
        (set `local.LowIndex` _array_index)
        (set `local.LowTransform` _returnvalue_4))))
  (`self.K2_SetActorTransform` (select `bool` (`local.NoInterp`) :`false` (`KismetMathLibrary.TInterpTo` (`self.GetTransform`) _returnvalue_3 (`local.Delta`) 1.0) :`true` _returnvalue_3)))

(fn `UserConstructionScript`)