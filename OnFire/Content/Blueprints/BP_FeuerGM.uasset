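; Game mode for a fire-based game that decides whether the fire is strong enough to lift a burnable object.
; On BeginPlay it caches the first BP_Fire actor found in the level.
; CanLiftBurnable divides a valid burnable's burning weight by the fire's strength, guarded against zero, and returns that ratio plus whether it falls under a fixed threshold.
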(event `self.ReceiveBeginPlay`
  (bind _outactors (`GameplayStatics.GetAllActorsOfClass` "/Game/Blueprints/BP_Fire.BP_Fire_C"))
  (set `self.FireRef` (`|GetArrayItem` _outactors)))

(fn `CanLiftBurnable`
  (params (Burnable :type "/Game/Blueprints/Burnables/BP_BurnableMain Object Reference"))
  (returns (CanLift :type Boolean) (Ratio :type "Float (double-precision)"))
  (bind _burnoptions_burningwheight (break `/Game/Data/STR_BurnableStats` (`/Game/Blueprints/Burnables/BP_BurnableMain.BurnOptions` Burnable)))
  (bind _firestrength (`/Game/Blueprints/BP_Fire.FireStrength` (`self.FireRef`)))
  (bind _returnvalue (/ _burnoptions_burningwheight (select `bool` (== _firestrength 0.0) :`false` _firestrength :`true` 1e-05)))
  (`/Engine/EditorBlueprintResources/StandardMacros.IsValid` Burnable
    (:`Is Valid`
      (return (< _returnvalue 1.25) _returnvalue))))

(fn `UserConstructionScript`)