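; BP_Fire is a fire actor that grows the area of its fire trigger over time.
; Each Tick raises a clamped FireStrength value, taking about five seconds to go from empty to full.
; That strength drives linear interpolation of FireTrigger's uniform scale between MinScale and MaxScale, and lifts it along Z by an offset derived from MaxScale.
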(event `self.ReceiveTick`
  (params (DeltaSeconds :type "Float (single-precision)"))
  (bind _firetrigger (`self.FireTrigger`))
  (set `self.FireStrength` (`KismetMathLibrary.FClamp` (+ (`self.FireStrength`) (/ DeltaSeconds 5.0))))
  (`SceneComponent.K2_SetRelativeLocation` _firetrigger (`KismetMathLibrary.VLerp` (0.0 0.0 0.0) (`KismetMathLibrary.MakeVector` 0.0 0.0 (- (* (`self.MaxScale`) 50.0) 50.0)) (`self.FireStrength`)) false false)
  (`SceneComponent.SetRelativeScale3D` _firetrigger (`KismetMathLibrary.VLerp` (`KismetMathLibrary.Conv_DoubleToVector` (`self.MinScale`)) (`KismetMathLibrary.Conv_DoubleToVector` (`self.MaxScale`)) (`self.FireStrength`))))

(fn `UserConstructionScript`)