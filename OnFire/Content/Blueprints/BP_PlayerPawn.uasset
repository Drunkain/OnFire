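; Player pawn that lets the mouse hover-select, pick up and drag burnable objects.
; Each tick it validates the held object, traces under the cursor to select idle burnables, then updates the drag target.
; Left mouse press lifts the selection if it is liftable, and release drops it.
; Dragging projects the cursor ray at the object's distance, keeping its X fixed so movement stays in the Y-Z plane.
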(event `self.ReceiveTick`
  (params (DeltaSeconds :type "Float (single-precision)"))
  (`|ExecutionSequence`
    (:`then_0`
      (`self.ValidateHandledBurnable`))
    (:`then_1`
      (`self.CheckBurnables`))
    (:`then_2`
      (`self.UpdateHandledBurnable`))))

(event `Key|LeftMouseButton`
  (params (Key :type "Key Structure"))
  (bind _selectedburnable (`self.SelectedBurnable`))
  (bind _selectedburnable_2 (`self.SelectedBurnable`))
  ;[1 1 1] Mouse
  (:`Pressed`
    (`/Engine/EditorBlueprintResources/StandardMacros.IsValid` _selectedburnable_2
      (:`Is Valid`
        (if (`/Game/Blueprints/Burnables/BP_BurnableMain.Liftable` _selectedburnable_2)
          (set `self.Handling` true)
          (`/Game/Blueprints/Burnables/BP_BurnableMain.Dragged` _selectedburnable)))))
  (:`Released`
    (set `self.Handling` false)
    (`/Engine/EditorBlueprintResources/StandardMacros.IsValid` _selectedburnable_2
      (:`Is Valid`
        (`/Game/Blueprints/Burnables/BP_BurnableMain.Dropped` _selectedburnable)))))

(fn `CheckBurnables`
  (bind _selectedburnable (`self.SelectedBurnable`))
  (bind _selectedburnable_2 (`self.SelectedBurnable`))
  (bind (_worldlocation _worlddirection) (`PlayerController.DeprojectMousePositionToWorld` (`self.GetBPController`)))
  (`WidgetLayoutLibrary.GetMousePositionOnViewport`)
  (bind _outhit (`KismetSystemLibrary.LineTraceSingleForObjects` _worldlocation (+ _worldlocation (* _worlddirection 1000000.0)) (`|MakeArray` "ObjectTypeQuery7" :!type "EObjectTypeQuery Enum")))
  (if (`GameplayStatics.BreakHitResult` _outhit)
    (bind _asbp_burnable_main (cast `/Game/Blueprints/Burnables/BP_BurnableMain` (`.HitActor` (`GameplayStatics.BreakHitResult` _outhit))))
    (switch `/Game/Data/E_BurnableState` (`/Game/Blueprints/Burnables/BP_BurnableMain.BurnableState` _asbp_burnable_main)
      (:`NewEnumerator0`
        (if (not (`self.Handling`))
          (`|ExecutionSequence`
            (:`then_0`
              (`/Engine/EditorBlueprintResources/StandardMacros.IsValid` _selectedburnable_2
                (:`Is Valid`
                  (set `/Game/Blueprints/Burnables/BP_BurnableMain.Selected` false _selectedburnable_2))))
            (:`then_1`
              (bind _output_get (set `self.SelectedBurnable` _asbp_burnable_main))
              (set `/Game/Blueprints/Burnables/BP_BurnableMain.Selected` true _output_get))))))
    (else
      (`/Engine/EditorBlueprintResources/StandardMacros.IsValid` _selectedburnable
        (:`Is Valid`
          (set `/Game/Blueprints/Burnables/BP_BurnableMain.Selected` false _selectedburnable))))))

(fn `GetBPController`
  (returns (NewParam :type "/Game/Blueprints/BP_PlayerController Object Reference"))
  (bind _asbp_player_controller (cast `/Game/Blueprints/BP_PlayerController` (`self.GetController`)))
  (return _asbp_player_controller))

(fn `GetCamera`
  (returns (CameraManager :type "/Game/Blueprints/BP_CameraManager Object Reference"))
  (bind _asbp_camera_manager (cast `/Game/Blueprints/BP_CameraManager` (`GameplayStatics.GetPlayerCameraManager` 0)))
  (return _asbp_camera_manager))

(fn `GetGM`
  (returns (GM :type "/Game/Blueprints/BP_FeuerGM Object Reference"))
  (bind _asbp_feuer_gm (cast `/Game/Blueprints/BP_FeuerGM` (`GameplayStatics.GetGameMode`))
    (:`then`
      (return _asbp_feuer_gm))
    (:`CastFailed`
      (`KismetSystemLibrary.PrintString` "CANT FIND GAMEMODE" true true (struct :`R` 1.0 :`G` 0.09104 :`A` 1.0)))))

(fn `UpdateHandledBurnable`
  (bind _selectedburnable (`self.SelectedBurnable`))
  (bind _returnvalue_x (`KismetMathLibrary.BreakVector` (`self.K2_GetActorLocation` _selectedburnable)))
  (bind (_worldlocation _worlddirection) (`PlayerController.DeprojectMousePositionToWorld` (`self.GetBPController`)))
  (bind (_returnvalue_x_2 _returnvalue_y _returnvalue_z) (`KismetMathLibrary.BreakVector` (+ _worldlocation (* _worlddirection (`KismetMathLibrary.Vector_Distance` (`self.K2_GetActorLocation` _selectedburnable) _worldlocation)))))
  (if (`self.Handling`)
    (`/Engine/EditorBlueprintResources/StandardMacros.IsValid` _selectedburnable
      (:`Is Valid`
        (if (`|EnumEquality` (`/Game/Blueprints/Burnables/BP_BurnableMain.BurnableState` _selectedburnable) "NewEnumerator2")
          (set `/Game/Blueprints/Burnables/BP_BurnableMain.TargetLocation` (`KismetMathLibrary.MakeVector` _returnvalue_x _returnvalue_y _returnvalue_z) _selectedburnable))))))

(fn `UserConstructionScript`)

(fn `ValidateHandledBurnable`
  (bind _selectedburnable (`self.SelectedBurnable`))
  (if (`self.Handling`)
    (`/Engine/EditorBlueprintResources/StandardMacros.IsValid` _selectedburnable
      (:`Is Valid`
        (set `self.Handling` (`/Game/Blueprints/Burnables/BP_BurnableMain.Liftable` _selectedburnable)))
      (:`Is Not Valid`
        (set `self.Handling` false)))))