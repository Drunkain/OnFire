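; BP_BurnableMain is a physics object that can be dragged, dropped and burned, destroying itself once BurnRatio reaches 1.
; A state enum switches between idle and handled; while handled, force and distance-scaled velocity damping pull it toward TargetLocation.
; Each tick it asks BP_FeuerGM whether it can be lifted, with a looser ratio threshold once liftable.
; Dynamic material instances display eased selection highlight, liftability and burn progress.
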(event `self.ReceiveBeginPlay`
  (for (_array_element _array_index) (`MeshComponent.GetMaterials` (`self.StaticMesh`))
    (bind _returnvalue (`PrimitiveComponent.CreateDynamicMaterialInstance` (`self.StaticMesh`) _array_index _array_element "None"))
    (`KismetArrayLibrary.Array_Add` (`self.MaterialInstances`) _returnvalue)))

(event `self.ReceiveTick`
  (params (DeltaSeconds :type "Float (single-precision)"))
  (bind _returnvalue (`GameplayStatics.GetWorldDeltaSeconds`))
  (bind _staticmesh (`self.StaticMesh`))
  (bind (_canlift _ratio) (`/Game/Blueprints/BP_FeuerGM.CanLiftBurnable` (`self.GetGM`) self))
  (`/Engine/EditorBlueprintResources/StandardMacros.IsValid` _staticmesh
    (:`Is Valid`
      (`PrimitiveComponent.SetEnableGravity` _staticmesh (select `/Game/Data/E_BurnableState` (`self.BurnableState`) :`NewEnumerator0` true :`NewEnumerator1` true :`NewEnumerator2` true))
      (`|ExecutionSequence`
        (:`then_0`
          (if (>= (`self.BurnRatio`) 1.0)
            (`self.OnBurn`)))
        (:`then_1`
          (switch `/Game/Data/E_BurnableState` (`self.BurnableState`)
            (:`NewEnumerator2`
              (`self.HandleHandling` _returnvalue))))
        (:`then_2`
          (`self.UpdateMaterial` _returnvalue))
        (:`then_3`
          (set `self.Liftable` (select `bool` (`self.Liftable`) :`false` _canlift :`true` (< _ratio 1.5))))))))

(fn `Dragged`
  (`self.SetBurnableState` "NewEnumerator2"))

(fn `Dropped`
  (`self.SetBurnableState` "NewEnumerator0"))

(fn `GetGM`
  (returns (GM :type "/Game/Blueprints/BP_FeuerGM Object Reference"))
  (bind _asbp_feuer_gm (cast `/Game/Blueprints/BP_FeuerGM` (`GameplayStatics.GetGameMode`)))
  (return _asbp_feuer_gm))

(fn `HandleHandling`
  (params (Delta :type "Float (double-precision)"))
  (bind _returnvalue (- (`self.TargetLocation`) (`self.K2_GetActorLocation`)))
  (bind _returnvalue_2 (`KismetMathLibrary.VSize` _returnvalue))
  (bind (_returnvalue_x _returnvalue_y _returnvalue_z) (`KismetMathLibrary.BreakVector` (* (`KismetMathLibrary.Normal` _returnvalue) (* (+ (* _returnvalue_2 50.0) 100.0) 100.0))))
  (bind _returnvalue_3 (`PrimitiveComponent.GetPhysicsLinearVelocity` (`self.StaticMesh`) "None"))
  (`PrimitiveComponent.SetPhysicsLinearVelocity` (`self.StaticMesh`) (`KismetMathLibrary.VInterpTo` _returnvalue_3 (* _returnvalue_3 (`KismetMathLibrary.MapRangeClamped` _returnvalue_2 0.0 1000.0 0.0 0.85)) (`GameplayStatics.GetWorldDeltaSeconds`) 10.0) false "None")
  (`PrimitiveComponent.AddForce` (`self.StaticMesh`) (* (`KismetMathLibrary.MakeVector` _returnvalue_x _returnvalue_y _returnvalue_z) (`local.Delta`)) "None" true))

(fn `OnBurn`
  (`|ExecutionSequence`
    (:`then_0`
      (`self.SetBurnableState` "NewEnumerator1"))
    (:`then_1`
      (`self.K2_DestroyActor`))))

(fn `SetBurnableState`
  (params (NewState :type "/Game/Data/E_BurnableState Enum" :default "NewEnumerator0"))
  (set `self.BurnableState` NewState))

(fn `UpdateMaterial`
  (params (Delta :type "Float (double-precision)"))
  (locals (SelectedParamName :type Name :default "Selected") (BurningParamName :type Name :default "Burning_Factor") (CanLiftParamName :type Name :default "CanLift"))
  (for _array_element (`self.MaterialInstances`)
    (bind _returnvalue (`MaterialInstanceDynamic.K2_GetScalarParameterValue` _array_element (`local.SelectedParamName`)))
    (`MaterialInstanceDynamic.SetScalarParameterValue` _array_element (`local.SelectedParamName`) (`KismetMathLibrary.FInterpTo` _returnvalue (select `bool` (`self.Selected`) :`true` (`KismetMathLibrary.Conv_BoolToDouble` (< (`.Ratio` (`/Game/Blueprints/BP_FeuerGM.CanLiftBurnable` (`self.GetGM`) self)) 1.5))) (`local.Delta`) 5.0))
    (`MaterialInstanceDynamic.SetScalarParameterValue` _array_element (`local.CanLiftParamName`) (`KismetMathLibrary.Conv_BoolToDouble` (`self.Liftable`)))
    (`MaterialInstanceDynamic.SetScalarParameterValue` _array_element (`local.BurningParamName`) (`self.BurnRatio`))))

(fn `UserConstructionScript`)